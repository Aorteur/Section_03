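; Openable door Blueprint that either rotates or slides when its OpenDoor open and close events fire.
; BeginPlay caches the initial transform and sets the rotation or location multiplier according to DoorType.
; The DoorSwing timeline plays or reverses, offsetting the transform along DoorAxis by DoorDistance through one shared formula masked by those multipliers.
; A timeline event track plays the lock sound at the door.
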(event `self.ReceiveBeginPlay`
  (set `self.InitialRotation` (`self.K2_GetActorRotation`))
  (set `self.InitialPosition` (`self.K2_GetActorLocation`))
  (switch `string` (`self.DoorType`)
    (:`Rotation`
      (set `self.RotationMultiply` 1.0))
    (:`Location`
      (set `self.LocationMultiply` 1.0))))

(event `self.OpenDoor.OnOpen`
  (bind _dooraxis (`self.DoorAxis`))
  ;[1 1 1] Open Door Event
  (bind (_direction _doormotion) (`Timeline|Door Swing` :!label _label)
    (:`Update`
      (`self.K2_SetActorLocationAndRotation` (+ (* _dooraxis (* _doormotion (`self.LocationMultiply`) (`self.DoorDistance`))) (`self.InitialPosition`)) (`KismetMathLibrary.ComposeRotators` (`self.InitialRotation`) (`KismetMathLibrary.MakeRotator` (.x (* _dooraxis (* _doormotion (`self.RotationMultiply`) (`self.DoorDistance`)))) (.y (* _dooraxis (* _doormotion (`self.RotationMultiply`) (`self.DoorDistance`)))) (.z (* _dooraxis (* _doormotion (`self.RotationMultiply`) (`self.DoorDistance`))))))))
    (:`Sound TIming`
      (`GameplayStatics.PlaySoundAtLocation` "/Game/Audio/door-lock.door-lock" (`self.K2_GetActorLocation`)))))

(event `self.OpenDoor.OnClose`
  ;[1 1 1] Open Door Event
  (goto _label :!via `Reverse`))

(fn `UserConstructionScript`)